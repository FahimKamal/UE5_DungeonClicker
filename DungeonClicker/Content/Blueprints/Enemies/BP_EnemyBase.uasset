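; Base enemy for a click-to-damage game, drawn with flipbook sprites and showing name, level and health widgets.
; Clicking its capsule applies the player's cursor damage and spawns floating damage text.
; Damage updates the health bar and plays a hit animation, using stats and flipbooks looked up by enemy name.
; At zero health it plays a death animation, increments the GameMode's current level and destroys itself.
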(event `self.ReceiveBeginPlay`
  (bind _game_mode (message `/Game/Blueprints/Interfaces/BPI_GameMode.Get GameMode Ref` (`GameplayStatics.GetGameMode`)))
  (set `self.Game Mode` _game_mode)
  (bind _player (message `/Game/Blueprints/Interfaces/BPI_Player.Get Player Ref` (`GameplayStatics.GetPlayerCharacter` 0)))
  (set `self.Player` _player)
  (bind _playercontroller (message `/Game/Blueprints/Interfaces/BPI_PlayerController.GetPlayerControllerRef` (`GameplayStatics.GetPlayerController` 0)))
  (set `self.Player Controller` _playercontroller)
  (bind _aswb_enemy_info (cast `/Game/UI/WB_EnemyInfo` (`WidgetComponent.GetUserWidgetObject` (`self.EnemyInfoWidget`))))
  (`/Game/UI/WB_EnemyInfo.Update Enemy Info UI` _aswb_enemy_info (`self.Enemy Name`) (`/Game/Blueprints/GM_DungeonClicker.Current Level` (`self.Game Mode`)))
  (`self.Update Health` (`.Health_11_04FADA9745C5E3AF5E724D80F8896A80` (break `/Game/Blueprints/Structures/ST_EnemyInfo` (`/Game/Blueprints/Libraries/BP_FunctionLibrary.GetEnemyInfo` (`self.Enemy Name`))))))

(event `self.CapsuleComponent.OnClicked`
  (params (TouchedComponent :type "PrimitiveComponent Object Reference") (ButtonPressed :type "Key Structure"))
  (bind _cursor_damage (`/Game/Blueprints/BP_Player.Cursor Damage` (`self.Player`)))
  (if (not (`self.bIsDead`))
    (`GameplayStatics.ApplyDamage` self _cursor_damage)
    (`/Game/Blueprints/PC_DungeonClicker.Spawn Floating Text` (`self.Player Controller`) (`KismetStringLibrary.Conv_DoubleToString` _cursor_damage) (`self.K2_GetActorLocation`))))

(event `self.ReceiveAnyDamage`
  (params (Damage :type "Float (single-precision)") (DamageType :type "DamageType Object Reference") (InstigatedBy :type "Controller Object Reference") (DamageCauser :type "Actor Object Reference"))
  (bind _current_health (`self.Current Health`))
  (bind _returnvalue (`KismetMathLibrary.FClamp` (- _current_health Damage) 0.0 _current_health))
  (if (not (> _returnvalue 0.0))
    (set `self.bIsDead` true))
  (`KismetSystemLibrary.PrintString` (`KismetTextLibrary.Conv_TextToString` (`|FormatText` "Health: {Health}" _returnvalue)))
  (`self.Update Health` _returnvalue)
  (`self.Hit Effect`))

(event `Update Health`
  (params (`Current Health` :type "Float (double-precision)"))
  (set `self.Current Health` `Current Health`)
  (bind _aswb_health_bar (cast `/Game/UI/WB_HealthBar` (`WidgetComponent.GetUserWidgetObject` (`self.HealthBarwidget`))))
  (`/Game/UI/WB_HealthBar.Update Health UI` _aswb_health_bar (`self.Current Health`) (`.Health_11_04FADA9745C5E3AF5E724D80F8896A80` (break `/Game/Blueprints/Structures/ST_EnemyInfo` (`/Game/Blueprints/Libraries/BP_FunctionLibrary.GetEnemyInfo` (`self.Enemy Name`))))))

(event `Hit Effect`
  (bind ((`IdleAnim_14_E309CA134507AB9A18DD6DB78C12CDFC` _idleanim) (`HitAnim_16_3988809F466E8F2E2ECA688FCCD95B09` _hitanim)) (break `/Game/Blueprints/Structures/ST_EnemyInfo` (`/Game/Blueprints/Libraries/BP_FunctionLibrary.GetEnemyInfo` (`self.Enemy Name`))))
  (`PaperFlipbookComponent.SetFlipbook` (`self.Sprite`) _hitanim)
  (`KismetSystemLibrary.Delay` (`PaperFlipbookComponent.GetFlipbookLength` (`self.Sprite`)))
  (if (`self.bIsDead`)
    (`self.Death`)
    (else
      (`PaperFlipbookComponent.SetFlipbook` (`self.Sprite`) _idleanim))))

(event `Death`
  (bind _sprite (`self.Sprite`))
  (`PaperFlipbookComponent.SetFlipbook` _sprite (`.DeathAnim_18_434B675946596698B69A61AD11FA58A6` (break `/Game/Blueprints/Structures/ST_EnemyInfo` (`/Game/Blueprints/Libraries/BP_FunctionLibrary.GetEnemyInfo` (`self.Enemy Name`)))))
  (`KismetSystemLibrary.Delay` (`PaperFlipbookComponent.GetFlipbookLength` _sprite))
  (`/Game/Blueprints/GM_DungeonClicker.Increment Current Level` (`self.Game Mode`))
  (`self.K2_DestroyActor`))

(fn `UserConstructionScript`)