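; Player Blueprint for a clicker-style game that holds coins, purchased items and damage stats, and sets up input on BeginPlay.
; Purchases deduct a count-based cost, refresh the UI, spawn the item at GameMode-provided points, then raise cursor damage or recalculate total DPS.
; A looping timer hits the controller's spawned enemy with DPS scaled to the timer interval.
; Mouse clicks swap the cursor image.
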(event `self.ReceiveBeginPlay`
  (bind _returnvalue (pcsubsystem `EnhancedInputLocalPlayerSubsystem` (`self.Player Controller`)))
  ;[1 1 1] Event BeginPlay. Get ref to player Controller, gamemode. Update coin UI and start auto damage timer.
  (bind _playercontroller (message `/Game/Blueprints/Interfaces/BPI_PlayerController.GetPlayerControllerRef` (`GameplayStatics.GetPlayerController` 0)))
  (set `self.Player Controller` _playercontroller)
  (bind _game_mode (message `/Game/Blueprints/Interfaces/BPI_GameMode.Get GameMode Ref` (`GameplayStatics.GetGameMode`)))
  (set `self.Game Mode` _game_mode)
  ;;[1 1 1] Custom mouse cursor
  (`/Engine/EditorBlueprintResources/StandardMacros.IsValid` _returnvalue
    (:`Is Valid`
      (`EnhancedInputSubsystemInterface.AddMappingContext` _returnvalue "/Game/Blueprints/Player/Inputs/IMC_Default.IMC_Default" 0 (struct))
      (`/Game/UI/WB_Main.Update Coins Amount UI` (`/Game/Blueprints/PC_DungeonClicker.Main Widget` (`self.Player Controller`)) (`self.AmountOfCoins`))
      (`self.Auto Damage`))))

(event `EnhancedInput|/Game/Blueprints/Player/Inputs/IA_MouseClick`
  (params (ActionValue :type Boolean) (ElapsedSeconds :type "Float (double-precision)") (TriggeredSeconds :type "Float (double-precision)") (InputAction :type "InputAction Object Reference" :default "/Game/Blueprints/Player/Inputs/IA_MouseClick.IA_MouseClick"))
  (bind _mouse_cursor (`/Game/Blueprints/PC_DungeonClicker.Mouse Cursor` (`self.Player Controller`)))
  ;[1 1 1] Mouse State change function
  (:`Triggered`
    (`/Game/UI/WB_MouseCursor.Set Mouse Cursor Image` _mouse_cursor "NewEnumerator1"))
  (:`Completed`
    (`/Game/UI/WB_MouseCursor.Set Mouse Cursor Image` _mouse_cursor "NewEnumerator0")))

(event `Update Amount of Coins`
  (params (AmountOfCoins :type Integer) (bAdd :type Boolean))
  (bind _amountofcoins (`self.AmountOfCoins`))
  (bind _player_controller (`self.Player Controller`))
  ;[1 1 1] Update amount of coin of player on killing an enemy and purchaseing any item
  (bind _output_get (set `self.AmountOfCoins` (select `bool` bAdd :`false` (- _amountofcoins AmountOfCoins) :`true` (+ _amountofcoins AmountOfCoins))))
  (`/Game/UI/WB_Main.Update Coins Amount UI` (`/Game/Blueprints/PC_DungeonClicker.Main Widget` _player_controller) _output_get)
  (`/Game/Blueprints/PC_DungeonClicker.f_Update Item Buy Text Color` _player_controller))

(event `Purchase Item`
  (params (`Item Info` :type "/Game/Blueprints/Structures/ST_ItemInfo Structure") (`Item Card` :type "/Game/UI/WB_ShopItemCard Object Reference"))
  (bind ((`Name_2_33A19B4C421D9AC585DE06B55A0319B5` _name) (`EnumName_14_02CAE1034EF1D14ECCC282932520FF80` _enumname) (`Class_5_CAF0A1394838654B6A91908ADA0DCA94` _class) (`DPS_18_06B921BD4DE349B722E09F8745E4E0E8` _dps)) (break `/Game/Blueprints/Structures/ST_ItemInfo` `Item Info`))
  (bind _value (`BlueprintMapLibrary.Map_Find` (`self.ItemsBought`) _name))
  ;[1 1 1] Purchase Item function.
  (`self.Update Amount of Coins` (`self.f_Get Item Cost` `Item Info`))
  (`BlueprintMapLibrary.Map_Add` (`self.ItemsBought`) _name (+ _value 1))
  (`/Game/UI/WB_ShopItemCard.Update Items Bought UI` `Item Card`)
  (`/Game/Blueprints/PC_DungeonClicker.Spawn Item` (`self.Player Controller`) _class (`|GetArrayItem` (`/Game/Blueprints/GM_DungeonClicker.f_Get Item Spawn Points` (`self.Game Mode`) _enumname) (- _value 1)))
  (if (`|EnumEquality` _enumname "NewEnumerator10")
    (`self.f_Increase Cursor Damage` _dps)
    (else
      (`self.f_UpdateTotalDPS`))))

(event `Auto Damage`
  ;[1 1 1] Auto damage timer. Will be called at the start of the game.
  (bind _returnvalue (`KismetSystemLibrary.K2_SetTimer` null "f_AutoDamage" (`self.AutoDamageTimerTime`) true))
  (set `self.AutoDamageHandle` _returnvalue))

(fn `f_AutoDamage`
  (`GameplayStatics.ApplyDamage` (`/Game/Blueprints/PC_DungeonClicker.SpawnedEnemy` (`self.Player Controller`)) (/ (`self.TotalDPS`) (/ 1.0 (`self.AutoDamageTimerTime`))) null null "/Game/Blueprints/BP_AutoDamage.BP_AutoDamage_C"))

(fn `f_Does Player Have EnoughCoins`
  (params (`Item Cost` :type Integer))
  (returns (`bHas Enough Coin` :type Boolean))
  (return (>= (`self.AmountOfCoins`) `Item Cost`)))

(fn `f_Get Item Cost`
  (params (Item :type "/Game/Blueprints/Structures/ST_ItemInfo Structure"))
  (returns (`Item Cost` :type Integer))
  (bind ((`Name_2_33A19B4C421D9AC585DE06B55A0319B5` _name) (`EnumName_14_02CAE1034EF1D14ECCC282932520FF80` _enumname)) (break `/Game/Blueprints/Structures/ST_ItemInfo` Item))
  (bind (_mouseclick _lightfeather _torch _runeoftime _luckyrainbow _knighthelmet _orcskull _theprotector _grandwizardhat _crownofevil _kingscrown) (break `/Game/Blueprints/Structures/ST_ItemCost` (`/Game/Blueprints/Libraries/BP_FunctionLibrary.f_GetItemCost` (`BlueprintMapLibrary.Map_Find` (`self.ItemsBought`) _name))))
  (return (select `/Game/Blueprints/Enums/E_Items` _enumname :`NewEnumerator10` _mouseclick :`NewEnumerator0` _lightfeather :`NewEnumerator1` _torch :`NewEnumerator2` _runeoftime :`NewEnumerator3` _luckyrainbow :`NewEnumerator4` _knighthelmet :`NewEnumerator5` _orcskull :`NewEnumerator6` _theprotector :`NewEnumerator7` _grandwizardhat :`NewEnumerator8` _crownofevil :`NewEnumerator9` _kingscrown)))

(fn `f_Increase Cursor Damage`
  (params (`Damge To Add` :type "Float (double-precision)"))
  (set `self.Cursor Damage` (+ (`self.Cursor Damage`) `Damge To Add`)))

(fn `f_UpdateTotalDPS`
  (locals (LocalTotalDPS :type "Float (double-precision)"))
  (bind _keys (`BlueprintMapLibrary.Map_Keys` (`self.ItemsBought`)))
  (for (_array_element _array_index) _keys
    (bind _values (`BlueprintMapLibrary.Map_Values` (`self.ItemsBought`)))
    (set `local.LocalTotalDPS` (+ (`local.LocalTotalDPS`) (* (`|GetArrayItem` _values _array_index) (`.DPS_18_06B921BD4DE349B722E09F8745E4E0E8` (break `/Game/Blueprints/Structures/ST_ItemInfo` (`/Game/Blueprints/Libraries/BP_FunctionLibrary.f_GetItemInfo` _array_element)))))))
  (set `self.TotalDPS` (`local.LocalTotalDPS`)))

(fn `Get Player Ref`
  (returns (Player :type "/Game/Blueprints/Player/BP_Player Object Reference"))
  (return self))

(fn `UserConstructionScript`)