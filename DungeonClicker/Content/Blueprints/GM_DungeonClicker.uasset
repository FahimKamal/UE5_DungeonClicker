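; Game mode for a dungeon clicker that runs level progression, enemy spawning and the round timer.
; Each level's enemy is looked up from level and enemy info and spawned through the player controller at the enemy spawn point.
; A looping timer updates the main widget and, on reaching zero, restores the enemy's health and restarts the countdown.
; At start it expands each item spawn point actor into a grid of per-item locations, exposed by a getter.
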(event `self.ReceiveBeginPlay`
  (bind (_enemy_class _spawn_transform) (`self.f_Get Enemy To Spawn For Current Level`))
  (bind _returnvalue (`GameplayStatics.GetActorOfClass` "/Game/Blueprints/SpawnPoints/BP_EnemySpawnPoint.BP_EnemySpawnPoint_C"))
  (set `self.Enemy Spawn Point` _returnvalue)
  (bind _playercontroller (message `/Game/Blueprints/Interfaces/BPI_PlayerController.GetPlayerControllerRef` (`GameplayStatics.GetPlayerController` 0)))
  (bind _output_get (set `self.Player Controller` _playercontroller))
  (`self.f_Set Item Spawn Points`)
  (`/Game/Blueprints/PC_DungeonClicker.SpawnEnemy` _output_get _enemy_class _spawn_transform)
  (`self.Start Round Timer`))

(event `Increment Current Level`
  (bind (_enemy_class _spawn_transform) (`self.f_Get Enemy To Spawn For Current Level`))
  (bind _result (`/Engine/EditorBlueprintResources/StandardMacros.IncrementInt` (`self.Current Level`))
    (:`  `
      (if (<= _result (`self.Max Level`))
        (`/Game/Blueprints/PC_DungeonClicker.SpawnEnemy` (`self.Player Controller`) _enemy_class _spawn_transform)
        (`self.Start Round Timer`)))))

(event `Start Round Timer`
  (set `self.Current Round Timer` (`self.Initial Round Timer`))
  (bind _returnvalue (`KismetSystemLibrary.K2_SetTimerDelegate` (delegate `Round Timer Loop`) (`self.Round Timer Time`) true))
  (set `self.Round Timer Hadle` _returnvalue))

(event `Round Timer Loop`
  (bind _output_get (set `self.Current Round Timer` (`KismetMathLibrary.FClamp` (- (`self.Current Round Timer`) (`self.Round Timer Time`)) 0.0 (`self.Current Round Timer`))))
  (`/Game/UI/WB_Main.Update Timer UI` (`/Game/Blueprints/PC_DungeonClicker.Main Widget` (`self.Player Controller`)) _output_get)
  (if (== (`self.Current Round Timer`) 0.0)
    (`/Game/Blueprints/Enemies/BP_EnemyBase.Restore Health` (`/Game/Blueprints/PC_DungeonClicker.SpawnedEnemy` (`self.Player Controller`)))
    (set `self.Current Round Timer` (`self.Initial Round Timer`))))

(fn `f_Get Enemy To Spawn For Current Level`
  (returns (`Enemy Class` :type "/Game/Blueprints/Enemies/BP_EnemyBase Class Reference") (`Spawn Transform` :type "Transform Structure (by ref)"))
  (return (`.Class_5_F1A76BDE446EA86BB7EE77B531FC450C` (break `/Game/Blueprints/Structures/ST_EnemyInfo` (`/Game/Blueprints/Libraries/BP_FunctionLibrary.GetEnemyInfo` (`.EnemyName_6_3C88E92C4E54957351E5F2B9E690C12C` (break `/Game/Blueprints/Structures/ST_LevelInfo` (`/Game/Blueprints/Libraries/BP_FunctionLibrary.GetLevelInfo` (`self.Current Level`))))))) (`self.GetTransform` (`self.Enemy Spawn Point`))))

(fn `f_Get Item Spawn Points`
  (params (`Item Name` :type "/Game/Blueprints/Enums/E_Items Enum" :default "NewEnumerator0"))
  (returns (`Spawn Points` :type "Array of Vector Structure"))
  (return (select `/Game/Blueprints/Enums/E_Items` `Item Name` :`NewEnumerator0` (`self.Light Feather Spawn points`) :`NewEnumerator1` (`self.Torch Spawn points`) :`NewEnumerator2` (`self.Rune Of Time Spawn points`) :`NewEnumerator3` (`self.Lucky Rainbow Spawn points`) :`NewEnumerator4` (`self.Knight Helmet Spawn points`) :`NewEnumerator5` (`self.Orc Skull Spawn points`) :`NewEnumerator6` (`self.The Protector Spawn points`) :`NewEnumerator7` (`self.Grand Wizard Hat Spawn points`) :`NewEnumerator8` (`self.Crown Of Evil Spawn points`) :`NewEnumerator9` (`self.Kings Crown Spawn points`))))

(fn `f_Set Item Spawn Points`
  (locals (`Local Loop Last Index` :type Integer :default 9) (`Local Amount of Rows` :type Integer :default 2) (`Local Loop Counter` :type Integer) (`Local Z Axis Multiplier` :type Integer) (`Local Item Spawn Point` :type "Array of /Game/Blueprints/SpawnPoints/BP_ItemSpawnPoint Object Reference"))
  (bind _local_item_spawn_point (`local.Local Item Spawn Point`))
  (bind _outactors (`GameplayStatics.GetAllActorsOfClass` "/Game/Blueprints/SpawnPoints/BP_ItemSpawnPoint.BP_ItemSpawnPoint_C"))
  (bind _output_get (set `local.Local Item Spawn Point` _outactors))
  (if (> (`KismetArrayLibrary.Array_Length` _output_get) 0)
    (for _index (range (+ (`local.Local Loop Last Index`) 1)) :!label _label
      (`KismetArrayLibrary.Array_Add` (select `/Game/Blueprints/Enums/E_Items` (`/Game/Blueprints/SpawnPoints/BP_ItemSpawnPoint.Item` (`|GetArrayItem` (`local.Local Item Spawn Point`))) :`NewEnumerator0` (`self.Light Feather Spawn points`) :`NewEnumerator1` (`self.Torch Spawn points`) :`NewEnumerator2` (`self.Rune Of Time Spawn points`) :`NewEnumerator3` (`self.Lucky Rainbow Spawn points`) :`NewEnumerator4` (`self.Knight Helmet Spawn points`) :`NewEnumerator5` (`self.Orc Skull Spawn points`) :`NewEnumerator6` (`self.The Protector Spawn points`) :`NewEnumerator7` (`self.Grand Wizard Hat Spawn points`) :`NewEnumerator8` (`self.Crown Of Evil Spawn points`) :`NewEnumerator9` (`self.Kings Crown Spawn points`)) (`KismetMathLibrary.MakeVector` (+ (.x (`self.K2_GetActorLocation` (`|GetArrayItem` (`local.Local Item Spawn Point`)))) (* 10.0 _index)) (.y (`self.K2_GetActorLocation` (`|GetArrayItem` (`local.Local Item Spawn Point`)))) (- (.z (`self.K2_GetActorLocation` (`|GetArrayItem` (`local.Local Item Spawn Point`)))) (* 10.0 (`local.Local Z Axis Multiplier`)))))
      (if (== (`local.Local Loop Last Index`) _index)
        (bind _result (`/Engine/EditorBlueprintResources/StandardMacros.IncrementInt` (`local.Local Loop Counter`))
          (:`  `
            (if (< _result (`local.Local Amount of Rows`))
              (`/Engine/EditorBlueprintResources/StandardMacros.IncrementInt` (`local.Local Z Axis Multiplier`)
                (:`  `
                  (goto _label)))
              (else
                (`KismetArrayLibrary.Array_Remove` _local_item_spawn_point)
                (if (`KismetArrayLibrary.Array_IsNotEmpty` _local_item_spawn_point)
                  (set `local.Local Z Axis Multiplier` 0)
                  (set `local.Local Loop Counter` 0)
                  (goto _label))))))))))

(fn `Get GameMode Ref`
  (returns (`Game Mode` :type "/Game/Blueprints/GM_DungeonClicker Object Reference"))
  (return self))

(fn `UserConstructionScript`)