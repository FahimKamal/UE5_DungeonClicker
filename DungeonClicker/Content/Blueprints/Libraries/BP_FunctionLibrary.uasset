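; Blueprint function library that looks up game data for enemies, levels, items and item costs from their data tables.
; Enemy and item names become row names after a string Replace, while level numbers convert directly to row names.
; Item cost reads the row numbered one above the amount already bought, giving the next purchase's entry.
; Each function returns a row only when found, with no not-found handling.
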(fn `f_GetEnemyInfo`
  (params (`Enemy Name` :type String))
  (returns (EnemyInfo :type "/Game/Blueprints/Structures/ST_EnemyInfo Structure"))
  (bind _returnvalue (`|GetDataTableRow` "/Game/Blueprints/DataTables/DT_EnemyInfo.DT_EnemyInfo" (`KismetStringLibrary.Conv_StringToName` (`KismetStringLibrary.Replace` `Enemy Name` " ")))
    (:`then`
      (return _returnvalue))))

(fn `f_GetItemCost`
  (params (`Amount Of Item Bought` :type Integer))
  (returns (`Item Cost Info` :type "/Game/Blueprints/Structures/ST_ItemCost Structure"))
  (bind _returnvalue (`|GetDataTableRow` "/Game/Blueprints/DataTables/DT_ItemCost.DT_ItemCost" (`KismetStringLibrary.Conv_StringToName` (`KismetStringLibrary.Conv_IntToString` (+ `Amount Of Item Bought` 1))))
    (:`then`
      (return _returnvalue))))

(fn `f_GetItemInfo`
  (params (`Item Name` :type String))
  (returns (`Item Info` :type "/Game/Blueprints/Structures/ST_ItemInfo Structure"))
  (bind _returnvalue (`|GetDataTableRow` "/Game/Blueprints/DataTables/DT_ItemInfo.DT_ItemInfo" (`KismetStringLibrary.Conv_StringToName` (`KismetStringLibrary.Replace` `Item Name` " ")))
    (:`then`
      (return _returnvalue))))

(fn `f_GetLevelInfo`
  (params (Level :type Integer))
  (returns (`Level Info` :type "/Game/Blueprints/Structures/ST_LevelInfo Structure"))
  (bind _returnvalue (`|GetDataTableRow` "/Game/Blueprints/DataTables/DT_LevelInfo.DT_LevelInfo" (`KismetStringLibrary.Conv_StringToName` (`KismetStringLibrary.Conv_IntToString` Level)))
    (:`then`
      (return _returnvalue))))