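; Player controller for a dungeon clicker game that owns the main UI and spawns enemies, items, hit effects and floating text.
; On BeginPlay it caches the player pawn, shows the main widget, creates the shop tooltip and unlocks the first level card.
; Shop cards are built from the DT_ItemInfo data table, with buy buttons colored and enabled by whether the pawn's coins cover each item's cost.
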(event `self.ReceiveBeginPlay`
  (bind _player (message `/Game/Blueprints/Interfaces/BPI_Player.Get Player Ref` (`GameplayStatics.GetPlayerCharacter` 0)))
  (set `self.Player Pawn` _player)
  (`self.Show Hide Widget` "NewEnumerator0" true)
  (`self.Initialize Player`)
  (`self.Create Shop Item Cards`)
  (`self.Unlock Level` 1))

(event `Initialize Player`
  (bind _returnvalue (`|CreateWidget` "/Game/UI/WB_ShopToolTip.WB_ShopToolTip_C"))
  (set `self.WB_Shop Tooltip` _returnvalue))

(event `Show Hide Widget`
  (params (Widget :type "/Game/Blueprints/Enums/E_GameWidgets Enum" :default "NewEnumerator0") (Show :type Boolean))
  (if Show
    (`self.f_ShowWidget` Widget)
    (else
      (`self.f_HideWidget` Widget))))

(event `SpawnEnemy`
  (params (Enemy :type "Actor Class Reference") (SpawnTransform :type "Transform Structure"))
  (bind _returnvalue (`|SpawnActorFromClass` Enemy SpawnTransform "AdjustIfPossibleButAlwaysSpawn" "MultiplyWithRoot" null null))
  (bind _enemybase (message `/Game/Blueprints/Interfaces/BPI_EnemyBase.Get Enemy Base Ref` _returnvalue))
  (set `self.SpawnedEnemy` _enemybase))

(event `Spawn Item`
  (params (Class :type "Actor Class Reference") (Location :type "Vector Structure"))
  (`|SpawnActorFromClass` Class (`KismetMathLibrary.MakeTransform` Location) "AlwaysSpawn" "MultiplyWithRoot" null null))

(event `SpawnHitEffect`
  (`|SpawnActorFromClass` "/Game/Blueprints/BP_HitEffet.BP_HitEffet_C" (`KismetMathLibrary.Conv_VectorToTransform` (`self.DeprojectMousePositionToWorld`)) "AlwaysSpawn" "MultiplyWithRoot" null null))

(event `Spawn Floating Text`
  (params (Text :type String) (`Spawn Location` :type "Vector Structure"))
  (`|SpawnActorFromClass` "/Game/Blueprints/BP_FloatingText.BP_FloatingText_C" (`KismetMathLibrary.MakeTransform` (`KismetMathLibrary.MakeVector` (.x `Spawn Location`) 1.0 (+ (.z `Spawn Location`) 20.0))) "AlwaysSpawn" "MultiplyWithRoot" null Text null)
  (`self.SpawnHitEffect`))

(event `Create Shop Item Cards`
  (`KismetArrayLibrary.Array_Clear` (`self.Shop Item Cards`))
  (bind _outrownames (`DataTableFunctionLibrary.GetDataTableRowNames` "/Game/Blueprints/DataTables/DT_ItemInfo.DT_ItemInfo"))
  (for _array_element _outrownames
    (bind _returnvalue (`|CreateWidget` "/Game/UI/WB_ShopItemCard.WB_ShopItemCard_C" null (`/Game/Blueprints/Libraries/BP_FunctionLibrary.f_GetItemInfo` (`KismetStringLibrary.Conv_NameToString` _array_element))))
    (`KismetArrayLibrary.Array_Add` (`self.Shop Item Cards`) _returnvalue))
  (`self.Display Shop Item Cards`)
  (`self.f_Update Item Buy Text Color`))

(event `Display Shop Item Cards`
  (`PanelWidget.ClearChildren` (`/Game/UI/WB_Main.VB_ItemList` (`self.Main Widget`)))
  (for _array_element (`self.Shop Item Cards`)
    (`VerticalBox.AddChildToVerticalBox` (`/Game/UI/WB_Main.VB_ItemList` (`self.Main Widget`)) _array_element)))

(event `Unlock Level`
  (params (Level :type Integer))
  (bind _returnvalue (`|CreateWidget` "/Game/UI/WB_LevelCard.WB_LevelCard_C" null Level))
  (`VerticalBox.AddChildToVerticalBox` (`/Game/UI/WB_Main.VB_LevelList` (`self.Main Widget`)) _returnvalue))

(fn `f_HideWidget`
  (params (Widget :type "/Game/Blueprints/Enums/E_GameWidgets Enum" :default "NewEnumerator0"))
  (switch `/Game/Blueprints/Enums/E_GameWidgets` Widget
    (:`NewEnumerator0`
      (bind _main_widget (`self.Main Widget`)
        (:`then`
          (`Widget.RemoveFromParent` _main_widget))
        (:`else`)))))

(fn `f_ShowWidget`
  (params (Widget :type "/Game/Blueprints/Enums/E_GameWidgets Enum" :default "NewEnumerator0"))
  (switch `/Game/Blueprints/Enums/E_GameWidgets` Widget
    (:`NewEnumerator0`
      (`self.Main Widget`
        (:`then`
          _)
        (:`else`
          (bind _returnvalue (`|CreateWidget` "/Game/UI/WB_Main.WB_Main_C"))
          (bind _output_get (set `self.Main Widget` _returnvalue))))
      (`UserWidget.AddToViewport` _output_get 0))))

(fn `f_Update Item Buy Text Color`
  (bind _player_pawn (`self.Player Pawn`))
  (for _array_element (`self.Shop Item Cards`)
    (bind _returnvalue (> (`/Game/Blueprints/BP_Player.F Get Item Cost` _player_pawn (`/Game/UI/WB_ShopItemCard.Item Info` _array_element)) (`/Game/Blueprints/BP_Player.AmountOfCoins` _player_pawn)))
    (`TextBlock.SetColorAndOpacity` (`/Game/UI/WB_ShopItemCard.TXT_Buy` _array_element) (make `SlateColor` (`KismetMathLibrary.SelectColor` (struct :`R` 0.537255 :`G` 0.022103 :`B` 0.016759 :`A` 1.0) (struct :`R` 0.417759 :`G` 1.0 :`B` 0.067708 :`A` 1.0) _returnvalue)))
    (`Widget.SetIsEnabled` (`/Game/UI/WB_ShopItemCard.BTN_Buy` _array_element) (not _returnvalue))))

(fn `GetPlayerControllerRef`
  (returns (PlayerController :type "/Game/Blueprints/PC_DungeonClicker Object Reference"))
  (return self))

(fn `UserConstructionScript`)